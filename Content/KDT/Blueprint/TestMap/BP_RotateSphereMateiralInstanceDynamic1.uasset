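; Test actor that drives a dynamic material instance on its static mesh, as a material parameter exercise.
; The construction script creates the instance and applies the Color, Texture and UV variables to it.
; On BeginPlay, a timeline animates the B channel of the UV vector parameter, and a looping timer fires an empty ChangeColor event.
; The color-cycling MultiGate and the spin and satellite-orbit rotation logic are disconnected and never run.
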(event `ChangeColor`)

(event `self.ReceiveBeginPlay`
  (bind (_uv_r _uv_g _uv_b _uv_a) (break `LinearColor` (`self.UV`)))
  (`KismetSystemLibrary.K2_SetTimerDelegate` (delegate `ChangeColor`) 1.0 true)
  (`|ExecutionSequence`
    (:`then_0`
      (bind (_direction _value) (`Timeline|UVTimeline`)
        (:`Update`
          (bind _output_get (set `self.UV` (make `LinearColor` _uv_r _uv_g _value _uv_a)))
          (`MaterialInstanceDynamic.SetVectorParameterValue` (`self.MID_StaticMesh`) "UV" _output_get))))
    (:`then_1`
      (`KismetSystemLibrary.PrintString` "Hello"))))

(event `self.ReceiveTick`
  (params (DeltaSeconds :type "Float (single-precision)")))

(fn `UserConstructionScript`
  (bind _returnvalue (`PrimitiveComponent.CreateDynamicMaterialInstance` (`self.StaticMesh`) 0 null "None"))
  (`/Engine/EditorBlueprintResources/StandardMacros.IsValid` _returnvalue
    (:`Is Valid`
      (bind _output_get (set `self.MID_StaticMesh` _returnvalue))
      (`MaterialInstanceDynamic.SetVectorParameterValue` _output_get "Color" (`self.Color`))
      (`MaterialInstanceDynamic.SetTextureParameterValue` _output_get "Texture" (`self.Texture`))
      (`MaterialInstanceDynamic.SetVectorParameterValue` (`self.MID_StaticMesh`) "UV" (`self.UV`)))))