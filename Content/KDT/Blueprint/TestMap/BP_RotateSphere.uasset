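; BP_RotateSphere is a test-map actor that animates a spinning sphere with an orbiting, spinning satellite.
; Each Tick adds yaw to StaticMesh for its spin, to Scene1 to swing the satellite around, and to StaticMesh1 for the satellite's own spin.
; Scene1 acts as the orbit pivot, and each component has its own speed variable scaled by delta time for frame-rate-independent motion.
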(event `self.ReceiveBeginPlay`)

(event `self.ReceiveActorBeginOverlap`
  (params (OtherActor :type "Actor Object Reference")))

(event `self.ReceiveTick`
  (params (DeltaSeconds :type "Float (single-precision)"))
  (`|ExecutionSequence`
    (:`then_0`
      ;[1 1 1] Static Mesh가 자전한다.
      (`SceneComponent.K2_AddRelativeRotation` (`self.StaticMesh`) (`KismetMathLibrary.MakeRotator` 0.0 0.0 (* DeltaSeconds (`self.StaticMeshRotationSpeed`))) false false))
    (:`then_1`
      ;[1 1 1] Scene1을 회전시켜 위성(StaticMesh1)을 공전시킨다.
      (`SceneComponent.K2_AddRelativeRotation` (`self.Scene1`) (`KismetMathLibrary.MakeRotator` 0.0 0.0 (* (`GameplayStatics.GetWorldDeltaSeconds`) (`self.Scene1RotationSpeed`))) false false)
      ;[1 1 1] Static Mesh1이 자전한다.
      (`SceneComponent.K2_AddRelativeRotation` (`self.StaticMesh1`) (`KismetMathLibrary.MakeRotator` 0.0 0.0 (* (`GameplayStatics.GetWorldDeltaSeconds`) (`self.StaticMesh1RotationSpeed`))) false false))))

(fn `UserConstructionScript`)