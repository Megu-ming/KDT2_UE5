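; Test actor that spins a satellite mesh in orbit and sets up a dynamic sprite-texture material on its main mesh.
; The construction script creates the material instance and applies Color, Texture and UV parameters.
; Tick yaws Scene1 for the orbit and StaticMesh1 for its self-spin, scaled by delta time.
; A looping timer calls an empty ChangeColor; color cycling, UV timeline animation and main-mesh rotation are left disconnected.
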(event `ChangeColor`)

(event `self.ReceiveBeginPlay`
  (`KismetSystemLibrary.K2_SetTimerDelegate` (delegate `ChangeColor`) 1.0 true))

(event `self.ReceiveTick`
  (params (DeltaSeconds :type "Float (single-precision)"))
  (`|ExecutionSequence`
    (:`then_1`
      ;[1 1 1] Scene1를 회전 시켜서 위성(StaticMesh1)을 공전 시킨다
      (`SceneComponent.K2_AddLocalRotation` (`self.Scene1`) (`KismetMathLibrary.MakeRotator` 0.0 0.0 (* (`GameplayStatics.GetWorldDeltaSeconds`) (`self.Scene1RotationSpeed`))) false false)
      ;[1 1 1] StaticMesh1 자전
      (`SceneComponent.K2_AddLocalRotation` (`self.StaticMesh1`) (`KismetMathLibrary.MakeRotator` 0.0 0.0 (* (`GameplayStatics.GetWorldDeltaSeconds`) (`self.StaticMesh1RotationSpeed`))) false false))))

(fn `UserConstructionScript`
  (bind _returnvalue (`PrimitiveComponent.CreateDynamicMaterialInstance` (`self.StaticMesh`) 0 "/Game/KDT/Blueprint/TestMap/MT_SpriteTexture.MT_SpriteTexture" "None"))
  (`/Engine/EditorBlueprintResources/StandardMacros.IsValid` _returnvalue
    (:`Is Valid`
      (bind _output_get (set `self.MID_StaticMesh` _returnvalue))
      (`MaterialInstanceDynamic.SetVectorParameterValue` _output_get "Color" (`self.Color`))
      (`MaterialInstanceDynamic.SetTextureParameterValue` _output_get "Texture" (`self.Texture`))
      (`MaterialInstanceDynamic.SetVectorParameterValue` (`self.MID_StaticMesh`) "UV" (`self.UV`)))))