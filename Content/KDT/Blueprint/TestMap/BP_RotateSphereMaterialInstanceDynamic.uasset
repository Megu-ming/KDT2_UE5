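; Test actor with a spinning sphere and an orbiting, spinning satellite mesh, demonstrating dynamic material instances.
; The construction script creates a MID from MT_Color on the main mesh and applies its Color, Texture and UV parameters.
; Tick yaws both meshes and the satellite's pivot, Scene1, using delta-time-scaled speeds.
; BeginPlay plays a timeline animating the UV vector's blue channel and sets a one-shot timer into a color MultiGate, so only red is applied.
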(event `Change Color`
  (bind _mid_staticmesh (`self.MID StaticMesh`))
  (`|MultiGate` false
    (:`Out 0`
      (`MaterialInstanceDynamic.SetVectorParameterValue` _mid_staticmesh "Color" (struct :`R` 1.0 :`A` 1.0)))
    (:`Out 1`
      (`MaterialInstanceDynamic.SetVectorParameterValue` _mid_staticmesh "Color" (struct :`B` 1.0 :`A` 1.0)))
    (:`Out 2`
      (`MaterialInstanceDynamic.SetVectorParameterValue` _mid_staticmesh "Color" (struct :`G` 1.0 :`A` 1.0)))))

(event `self.ReceiveBeginPlay`
  (bind (_uv_r _uv_g _uv_b _uv_a) (break `LinearColor` (`self.UV`)))
  (`KismetSystemLibrary.K2_SetTimerDelegate` (delegate `Change Color`) 1.0)
  (bind (_direction _value) (`Timeline|UV타임라인`)
    (:`Update`
      (bind _output_get (set `self.UV` (make `LinearColor` _uv_r _uv_g _value _uv_a)))
      (`MaterialInstanceDynamic.SetVectorParameterValue` (`self.MID StaticMesh`) "UV" _output_get))))

(event `self.ReceiveActorBeginOverlap`
  (params (OtherActor :type "Actor Object Reference")))

(event `self.ReceiveTick`
  (params (DeltaSeconds :type "Float (single-precision)"))
  (`|ExecutionSequence`
    (:`then_0`
      ;[1 1 1] Static Mesh가 자전한다.
      (`SceneComponent.K2_AddRelativeRotation` (`self.StaticMesh`) (`KismetMathLibrary.MakeRotator` 0.0 0.0 (* (`GameplayStatics.GetWorldDeltaSeconds`) (`self.StaticMeshRotationSpeed`))) false false))
    (:`then_1`
      ;[1 1 1] Scene1을 회전시켜 위성(StaticMesh1)을 공전시킨다.
      (`SceneComponent.K2_AddRelativeRotation` (`self.Scene1`) (`KismetMathLibrary.MakeRotator` 0.0 0.0 (* (`GameplayStatics.GetWorldDeltaSeconds`) (`self.Scene1RotationSpeed`))) false false)
      ;[1 1 1] Static Mesh1이 자전한다.
      (`SceneComponent.K2_AddRelativeRotation` (`self.StaticMesh1`) (`KismetMathLibrary.MakeRotator` 0.0 0.0 (* (`GameplayStatics.GetWorldDeltaSeconds`) (`self.StaticMesh1RotationSpeed`))) false false))
    (:`then_2`)))

(fn `UserConstructionScript`
  (bind _returnvalue (`PrimitiveComponent.CreateDynamicMaterialInstance` (`self.StaticMesh`) 0 "/Game/KDT/Blueprint/TestMap/MT_Color.MT_Color" "None"))
  (`/Engine/EditorBlueprintResources/StandardMacros.IsValid` _returnvalue
    (:`Is Valid`
      (bind _output_get (set `self.MID StaticMesh` _returnvalue))
      (`MaterialInstanceDynamic.SetVectorParameterValue` _output_get "Color" (`self.Color`))
      (`MaterialInstanceDynamic.SetTextureParameterValue` _output_get "Texture" (`self.Texture`))
      (`MaterialInstanceDynamic.SetVectorParameterValue` (`self.MID StaticMesh`) "UV" (`self.UV`)))))