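; BP_Earth is a solar system Earth actor with spinning planet, cloud and moon pivots.
; Tick yaws the EarthAxis, CloudAxis and MoonAxis components at separate constant rates scaled by delta time.
; The construction script creates a dynamic material on the Earth mesh and feeds it a LightDirection vector pointing toward the Sun actor.
; That direction is computed only at construction, so Tick never updates it.
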(event `self.ReceiveTick`
  (params (DeltaSeconds :type "Float (single-precision)"))
  (`|ExecutionSequence`
    (:`then_0`
      (`SceneComponent.K2_AddLocalRotation` (`self.EarthAxis`) (`KismetMathLibrary.MakeRotator` 0.0 0.0 (* DeltaSeconds 90.0)) false false))
    (:`then_1`
      (`SceneComponent.K2_AddLocalRotation` (`self.CloudAxis`) (`KismetMathLibrary.MakeRotator` 0.0 0.0 (* DeltaSeconds 180.0)) false false))
    (:`then_2`
      (`SceneComponent.K2_AddLocalRotation` (`self.MoonAxis`) (`KismetMathLibrary.MakeRotator` 0.0 0.0 (* DeltaSeconds 60.0)) false false))))

(event `커스텀이벤트`)

(fn `UserConstructionScript`
  (bind _earth (`self.Earth`))
  (bind _returnvalue (`PrimitiveComponent.CreateDynamicMaterialInstance` _earth 0 (`PrimitiveComponent.GetMaterial` _earth 0) "None"))
  (bind _output_get (set `self.MID_Earth` _returnvalue))
  (`|ExecutionSequence`
    (:`then_0`
      (bind _returnvalue_2 (`GameplayStatics.GetActorOfClass` "/Script/KDT2.Sun"))
      (`/Engine/EditorBlueprintResources/StandardMacros.IsValid` _returnvalue_2
        (:`Is Valid`
          (set `self.SunLocation` (`self.K2_GetActorLocation` _returnvalue_2)))))
    (:`then_1`
      (set `self.LightDirection` (`KismetMathLibrary.GetDirectionUnitVector` (`self.K2_GetActorLocation`) (`self.SunLocation`))))
    (:`then_2`
      (`MaterialInstanceDynamic.SetVectorParameterValue` _output_get "LightDirection" (`KismetMathLibrary.Conv_VectorToLinearColor` (`self.LightDirection`))))))