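; Test actor that spins a sphere mesh with an orbiting, self-rotating satellite and animates the sphere's material.
; The construction script creates a dynamic instance of MT_SpriteTexture on the main mesh, seeded with color, texture and UV variables.
; A looping timer cycles its color through red, blue and green via MultiGate, while a timeline drives one UV component.
; Tick applies the rotations, orbiting the satellite by turning its parent scene component.
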(event `ChangeColor`
  (bind _mid_staticmesh (`self.MID_StaticMesh`))
  (`|MultiGate` false true
    (:`Out 0`
      (`MaterialInstanceDynamic.SetVectorParameterValue` _mid_staticmesh "Color" (struct :`R` 1.0 :`A` 1.0)))
    (:`Out 1`
      (`MaterialInstanceDynamic.SetVectorParameterValue` _mid_staticmesh "Color" (struct :`G` 0.125949 :`B` 1.0 :`A` 1.0)))
    (:`Out 2`
      (`MaterialInstanceDynamic.SetVectorParameterValue` _mid_staticmesh "Color" (struct :`R` 0.175088 :`G` 1.0 :`A` 1.0)))))

(event `self.ReceiveBeginPlay`
  (bind (_uv_r _uv_g _uv_b _uv_a) (break `LinearColor` (`self.UV`)))
  (`KismetSystemLibrary.K2_SetTimerDelegate` (delegate `ChangeColor`) 1.0 true)
  (bind (_direction _value) (`Timeline|UVTimeline`)
    (:`Update`
      (bind _output_get (set `self.UV` (make `LinearColor` _uv_r _uv_g _value _uv_a)))
      (`MaterialInstanceDynamic.SetVectorParameterValue` (`self.MID_StaticMesh`) "UV" _output_get))))

(event `self.ReceiveTick`
  (params (DeltaSeconds :type "Float (single-precision)"))
  (`|ExecutionSequence`
    (:`then_0`
      ;[1 1 1] StaticMesh를 회전 시킨다
      (`SceneComponent.K2_AddLocalRotation` (`self.StaticMesh`) (`KismetMathLibrary.MakeRotator` 0.0 (* DeltaSeconds (`self.StaticMeshRotationSpeed`))) false false))
    (:`then_1`
      ;[1 1 1] Scene1를 회전 시켜서 위성(StaticMesh1)을 공전 시킨다
      (`SceneComponent.K2_AddLocalRotation` (`self.Scene1`) (`KismetMathLibrary.MakeRotator` 0.0 0.0 (* (`GameplayStatics.GetWorldDeltaSeconds`) (`self.Scene1RotationSpeed`))) false false)
      ;[1 1 1] StaticMesh1 자전
      (`SceneComponent.K2_AddLocalRotation` (`self.StaticMesh1`) (`KismetMathLibrary.MakeRotator` 0.0 0.0 (* (`GameplayStatics.GetWorldDeltaSeconds`) (`self.StaticMesh1RotationSpeed`))) false false))))

(fn `UserConstructionScript`
  (bind _returnvalue (`PrimitiveComponent.CreateDynamicMaterialInstance` (`self.StaticMesh`) 0 "/Game/KDT2/Blueprint/TestMap/MT_SpriteTexture.MT_SpriteTexture" "None"))
  (`/Engine/EditorBlueprintResources/StandardMacros.IsValid` _returnvalue
    (:`Is Valid`
      (bind _output_get (set `self.MID_StaticMesh` _returnvalue))
      (`MaterialInstanceDynamic.SetVectorParameterValue` _output_get "Color" (`self.Color`))
      (`MaterialInstanceDynamic.SetTextureParameterValue` _output_get "Texture" (`self.Texture`))
      (`MaterialInstanceDynamic.SetVectorParameterValue` (`self.MID_StaticMesh`) "UV" (`self.UV`)))))