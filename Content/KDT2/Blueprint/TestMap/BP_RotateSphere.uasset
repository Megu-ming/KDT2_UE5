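; BP_RotateSphere is a test-map actor that animates a spinning sphere with an orbiting satellite.
; Each Tick pitches StaticMesh locally and yaws the Scene1 pivot to orbit StaticMesh1, which also spins on its own yaw.
; Each rotation has its own speed variable scaled by frame delta time for framerate independence.
; Construction and BeginPlay only print debug strings, and disconnected leftover nodes never run.
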(event `self.ReceiveBeginPlay`
  (`KismetSystemLibrary.PrintString` "BeginPlayer"))

(event `self.ReceiveTick`
  (params (DeltaSeconds :type "Float (single-precision)"))
  (`|ExecutionSequence`
    (:`then_0`
      ;[1 1 1] StaticMesh를 회전 시킨다
      (`SceneComponent.K2_AddLocalRotation` (`self.StaticMesh`) (`KismetMathLibrary.MakeRotator` 0.0 (* DeltaSeconds (`self.StaticMeshRotationSpeed`))) false false))
    (:`then_1`
      ;[1 1 1] Scene1를 회전 시켜서 위성(StaticMesh1)을 공전 시킨다
      (`SceneComponent.K2_AddLocalRotation` (`self.Scene1`) (`KismetMathLibrary.MakeRotator` 0.0 0.0 (* (`GameplayStatics.GetWorldDeltaSeconds`) (`self.Scene1RotationSpeed`))) false false)
      ;[1 1 1] StaticMesh1 자전
      (`SceneComponent.K2_AddLocalRotation` (`self.StaticMesh1`) (`KismetMathLibrary.MakeRotator` 0.0 0.0 (* (`GameplayStatics.GetWorldDeltaSeconds`) (`self.StaticMesh1RotationSpeed`))) false false))))

(fn `UserConstructionScript`
  (`KismetSystemLibrary.PrintString` "Hello"))