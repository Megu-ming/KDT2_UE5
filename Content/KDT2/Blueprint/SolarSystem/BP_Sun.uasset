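; BP_Sun is the sun actor in the solar system, animating the power of its material.
; The construction script creates a dynamic material instance from the static mesh's first material and stores it as MIDSun.
; On BeginPlay, the SunPower timeline plays at half speed, writing its scaled track value to the material's Power parameter on each update.
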(event `self.ReceiveBeginPlay`
  (`TimelineComponent.SetPlayRate` (`self.SunPower`) 0.5)
  (bind (_direction _power) (`Timeline|SunPower`)
    (:`Update`
      (`MaterialInstanceDynamic.SetScalarParameterValue` (`self.MID_Sun`) "Power" (* _power 50.0)))))

(fn `UserConstructionScript`
  (bind _staticmesh (`self.StaticMesh`))
  (bind _returnvalue (`PrimitiveComponent.CreateDynamicMaterialInstance` _staticmesh 0 (`PrimitiveComponent.GetMaterial` _staticmesh 0) "None"))
  (set `self.MID_Sun` _returnvalue))