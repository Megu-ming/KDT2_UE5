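; BPPC_Tank is the player controller that turns player input into actions on the controlled tank pawn.
; On BeginPlay it adds the IMC_Tank Enhanced Input mapping context.
; Zoom start and completion call ZoomIn and ZoomOut on the pawn cast to BP_Tank, and the fire action calls Fire the same way.
; The tank implements the actions itself, and the controller only forwards input.
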(event `self.ReceiveBeginPlay`
  (`EnhancedInputSubsystemInterface.AddMappingContext` (subsystem `EnhancedInputLocalPlayerSubsystem`) "/Game/KDT2/Blueprint/Tank/Input/IMC_Tank.IMC_Tank" 0 (struct)))

(event `EnhancedInput|/Game/KDT2/Blueprint/Tank/Input/IA_Zoom`
  (params (ActionValue :type Boolean) (ElapsedSeconds :type "Float (double-precision)") (TriggeredSeconds :type "Float (double-precision)") (InputAction :type "InputAction Object Reference" :default "/Game/KDT2/Blueprint/Tank/Input/IA_Zoom.IA_Zoom"))
  (bind _returnvalue (`self.K2_GetPawn`))
  (:`Started`
    (bind _asbp_tank (cast `/Game/KDT2/Blueprint/Tank/BP_Tank` _returnvalue))
    (`/Game/KDT2/Blueprint/Tank/BP_Tank.ZoomIn` _asbp_tank))
  (:`Completed`
    (bind _asbp_tank_2 (cast `/Game/KDT2/Blueprint/Tank/BP_Tank` _returnvalue))
    (`/Game/KDT2/Blueprint/Tank/BP_Tank.ZoomOut` _asbp_tank_2)))

(event `EnhancedInput|/Game/KDT2/Blueprint/Tank/Input/IA_Fire`
  (params (ActionValue :type Boolean) (ElapsedSeconds :type "Float (double-precision)") (TriggeredSeconds :type "Float (double-precision)") (InputAction :type "InputAction Object Reference" :default "/Game/KDT2/Blueprint/Tank/Input/IA_Fire.IA_Fire"))
  (:`Triggered`
    (bind _asbp_tank (cast `/Game/KDT2/Blueprint/Tank/BP_Tank` (`self.K2_GetPawn`)))
    (`/Game/KDT2/Blueprint/Tank/BP_Tank.Fire` _asbp_tank)))

(fn `UserConstructionScript`)