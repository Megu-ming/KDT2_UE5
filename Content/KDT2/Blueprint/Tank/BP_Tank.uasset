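; BP_Tank is a player-controlled tank Blueprint with a zoom view and a placeholder fire action.
; BeginPlay creates the UI_TankZoomIn widget for the controlling player and starts zoomed out.
; ZoomIn and ZoomOut toggle between the main and zoom cameras, adding or removing that widget.
; Fire only prints a debug message, using a boolean and short Delay as a cooldown gate.
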(event `self.ReceiveBeginPlay`
  (`|ExecutionSequence`
    (:`then_0`
      (bind `_as플레이어_컨트롤러` (cast `PlayerController` (`self.GetController`)))
      (bind _returnvalue (`|CreateWidget` "/Game/KDT2/Blueprint/Tank/UI/UI_TankZoomIn.UI_TankZoomIn_C" `_as플레이어_컨트롤러`))
      (set `self.UI_TankZoomIn` _returnvalue))
    (:`then_1`
      (`self.ZoomOut`))))

(event `Fire`
  (if (`self.bFire`)
    (set `self.bFire` false)
    (`KismetSystemLibrary.PrintString` "Fire!" true true (struct :`R` 1.0 :`A` 1.0))
    (`KismetSystemLibrary.Delay` 0.2)
    (set `self.bFire` true)))

(fn `UserConstructionScript`)

(fn `ZoomIn`
  (`ActorComponent.SetActive` (`self.ZoomCamera`) true false)
  (`ActorComponent.SetActive` (`self.Camera`) false false)
  (`UserWidget.AddToViewport` (`self.UI_TankZoomIn`) 0))

(fn `ZoomOut`
  (`ActorComponent.SetActive` (`self.ZoomCamera`) false false)
  (`ActorComponent.SetActive` (`self.Camera`) true false)
  (`Widget.RemoveFromParent` (`self.UI_TankZoomIn`)))