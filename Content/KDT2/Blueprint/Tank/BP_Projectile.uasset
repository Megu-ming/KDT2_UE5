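; BP_Projectile is a projectile in the Tank folder that flies forward and destroys itself on impact.
; The construction script applies Speed to the ProjectileMovement component, while Tick also moves the actor along its forward vector with a swept move.
; A valid sweep hit actor or a Hit event destroys it, with the latter printing the other object's name.
; BeginPlay stores BP_Tank's muzzle forward vector in StartingPoint, unused in these graphs.
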(event `self.ReceiveBeginPlay`
  (bind _returnvalue (`GameplayStatics.GetActorOfClass` "/Game/KDT2/Blueprint/Tank/BP_Tank.BP_Tank_C"))
  (set `self.StartingPoint` (`SceneComponent.GetForwardVector` (`/Game/KDT2/Blueprint/Tank/BP_Tank.Muzzle` _returnvalue))))

(event `self.ReceiveTick`
  (params (DeltaSeconds :type "Float (single-precision)"))
  (bind _sweephitresult (`self.K2_SetActorLocation` (+ (`self.K2_GetActorLocation`) (* (`SceneComponent.GetForwardVector` (`self.RootComponent`)) (`self.Speed`) DeltaSeconds)) true))
  (`/Engine/EditorBlueprintResources/StandardMacros.IsValid` (`.HitActor` (`GameplayStatics.BreakHitResult` _sweephitresult))
    (:`Is Valid`
      (`self.K2_DestroyActor`))))

(event `self.ReceiveHit`
  (params (MyComp :type "PrimitiveComponent Object Reference") (Other :type "Actor Object Reference") (OtherComp :type "PrimitiveComponent Object Reference") (bSelfMoved :type Boolean) (HitLocation :type "Vector Structure") (HitNormal :type "Vector Structure") (NormalImpulse :type "Vector Structure") (Hit :type "HitResult Structure (by ref)"))
  (`self.K2_DestroyActor`)
  (`KismetSystemLibrary.PrintString` (`KismetSystemLibrary.GetDisplayName` Other)))

(fn `UserConstructionScript`
  (bind _projectilemovement (`self.ProjectileMovement`))
  (bind _speed (`self.Speed`))
  (set `ProjectileMovementComponent.InitialSpeed` _speed _projectilemovement)
  (set `ProjectileMovementComponent.MaxSpeed` _speed _projectilemovement))