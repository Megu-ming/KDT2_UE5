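; BP_PortalTrigger is a lobby trigger actor that carries a BP_Portal as a child actor and configures its destination level and appearance.
; After running the parent construction script, it copies its Level, Power and Color to the child portal, then refreshes the portal's widget name and dynamic material.
; The event graph holds only empty event stubs, so this Blueprint adds no runtime logic of its own.
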(fn `UserConstructionScript`
  (`parent.UserConstructionScript`)
  (bind _asbp_portal (cast `/Game/KDT2/Blueprint/Lobby/Trigger/BP_Portal` (`ChildActorComponent.ChildActor` (`self.ChildActor`))))
  (set `/Game/KDT2/Blueprint/Lobby/Trigger/BP_Portal.Level` (`self.Level`) _asbp_portal)
  (`/Game/KDT2/Blueprint/Lobby/Trigger/BP_Portal.SetWidgetName` _asbp_portal)
  (set `/Game/KDT2/Blueprint/Lobby/Trigger/BP_Portal.Power` (`self.Power`) _asbp_portal)
  (set `/Game/KDT2/Blueprint/Lobby/Trigger/BP_Portal.Color` (`self.Color`) _asbp_portal)
  (`/Game/KDT2/Blueprint/Lobby/Trigger/BP_Portal.UpdateMID` _asbp_portal))