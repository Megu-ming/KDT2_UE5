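; BP_Trigger is a lobby trigger actor that relays overlap events to the actor held in its ChildActor component.
; Begin and end overlaps on CollisionComponent call the child's BPI_Trigger trigger functions, while those on Sphere call the inner-trigger variants, giving two detection zones.
; Each relay passes the overlapping actor along and does nothing if the child does not implement BPI_Trigger, keeping the response logic in the child.
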(event `self.CollisionComponent.OnComponentBeginOverlap`
  (params (OverlappedComponent :type "PrimitiveComponent Object Reference") (OtherActor :type "Actor Object Reference") (OtherComp :type "PrimitiveComponent Object Reference") (OtherBodyIndex :type Integer) (bFromSweep :type Boolean) (SweepResult :type "HitResult Structure (by ref)"))
  (bind _asbpi_trigger (cast `/Game/KDT2/Blueprint/Lobby/Trigger/BPI_Trigger` (`ChildActorComponent.ChildActor` (`self.ChildActor`))))
  (`/Game/KDT2/Blueprint/Lobby/Trigger/BPI_Trigger.OnTriggerBeginOverlap` _asbpi_trigger OtherActor))

(event `self.CollisionComponent.OnComponentEndOverlap`
  (params (OverlappedComponent :type "PrimitiveComponent Object Reference") (OtherActor :type "Actor Object Reference") (OtherComp :type "PrimitiveComponent Object Reference") (OtherBodyIndex :type Integer))
  (bind _asbpi_trigger (cast `/Game/KDT2/Blueprint/Lobby/Trigger/BPI_Trigger` (`ChildActorComponent.ChildActor` (`self.ChildActor`))))
  (`/Game/KDT2/Blueprint/Lobby/Trigger/BPI_Trigger.OnTriggerEndOverlap` _asbpi_trigger OtherActor))

(event `self.Sphere.OnComponentBeginOverlap`
  (params (OverlappedComponent :type "PrimitiveComponent Object Reference") (OtherActor :type "Actor Object Reference") (OtherComp :type "PrimitiveComponent Object Reference") (OtherBodyIndex :type Integer) (bFromSweep :type Boolean) (SweepResult :type "HitResult Structure (by ref)"))
  (bind _asbpi_trigger (cast `/Game/KDT2/Blueprint/Lobby/Trigger/BPI_Trigger` (`ChildActorComponent.ChildActor` (`self.ChildActor`))))
  (`/Game/KDT2/Blueprint/Lobby/Trigger/BPI_Trigger.OnInnerTriggerBeginOverlap` _asbpi_trigger OtherActor))

(event `self.Sphere.OnComponentEndOverlap`
  (params (OverlappedComponent :type "PrimitiveComponent Object Reference") (OtherActor :type "Actor Object Reference") (OtherComp :type "PrimitiveComponent Object Reference") (OtherBodyIndex :type Integer))
  (bind _asbpi_trigger (cast `/Game/KDT2/Blueprint/Lobby/Trigger/BPI_Trigger` (`ChildActorComponent.ChildActor` (`self.ChildActor`))))
  (`/Game/KDT2/Blueprint/Lobby/Trigger/BPI_Trigger.OnInnerTriggerEndOverlap` _asbpi_trigger OtherActor))

(fn `UserConstructionScript`)