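; Player controller for the lobby that handles mouse look and pawn movement through Enhanced Input.
; On BeginPlay it adds the lobby mapping context and clamps camera pitch to a limited range above and below level.
; Look input feeds controller yaw and pitch.
; Move input drives the controlled pawn along forward and right vectors built only from the controller's actor yaw, keeping movement independent of pitch.
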(event `self.ReceiveBeginPlay`
  (bind _playercameramanager (`self.PlayerCameraManager`))
  (`EnhancedInputSubsystemInterface.AddMappingContext` (subsystem `EnhancedInputLocalPlayerSubsystem`) "/Game/KDT2/Blueprint/Lobby/Input/IMC_Lobby.IMC_Lobby" 0 (struct))
  (set `PlayerCameraManager.ViewPitchMax` 40.0 _playercameramanager)
  (set `PlayerCameraManager.ViewPitchMin` -40.0 _playercameramanager))

(event `EnhancedInput|/Game/KDT2/Blueprint/Lobby/Input/IA_LookMouse`
  (params (ActionValue :type "Vector2D Structure") (ElapsedSeconds :type "Float (double-precision)") (TriggeredSeconds :type "Float (double-precision)") (InputAction :type "InputAction Object Reference" :default "/Game/KDT2/Blueprint/Lobby/Input/IA_LookMouse.IA_LookMouse"))
  (:`Triggered`
    (`self.AddYawInput` ActionValue_X)
    (`self.AddPitchInput` ActionValue_Y)))

(event `EnhancedInput|/Game/KDT2/Blueprint/Lobby/Input/IA_Move`
  (params (ActionValue :type "Vector2D Structure") (ElapsedSeconds :type "Float (double-precision)") (TriggeredSeconds :type "Float (double-precision)") (InputAction :type "InputAction Object Reference" :default "/Game/KDT2/Blueprint/Lobby/Input/IA_Move.IA_Move"))
  (bind _returnvalue (`self.K2_GetPawn`))
  (bind (_returnvalue_roll _returnvalue_pitch _returnvalue_yaw) (`KismetMathLibrary.BreakRotator` (`self.K2_GetActorRotation`)))
  (:`Triggered`
    (`Pawn.AddMovementInput` _returnvalue (`KismetMathLibrary.GetForwardVector` (`KismetMathLibrary.MakeRotator` 0.0 0.0 _returnvalue_yaw)) ActionValue_Y false)
    (`Pawn.AddMovementInput` _returnvalue (`KismetMathLibrary.GetRightVector` (`KismetMathLibrary.MakeRotator` 0.0 0.0 _returnvalue_yaw)) ActionValue_X false)))

(fn `UserConstructionScript`)