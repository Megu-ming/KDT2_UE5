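; BP_Tank is a player-controllable tank that fires projectiles and switches between a normal and a zoom camera.
; BeginPlay creates the zoom-in UI widget for its player controller, then starts zoomed out.
; ZoomIn and ZoomOut toggle the two cameras and add or remove that widget.
; Fire spawns BP_Projectile at the Scene component's location and rotation, using a boolean and Delay as a cooldown.
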(event `self.ReceiveBeginPlay`
  (`|ExecutionSequence`
    (:`then_0`
      (bind `_as플레이어_컨트롤러` (cast `PlayerController` (`self.GetController`)))
      (bind _returnvalue (`|CreateWidget` "/Game/KDT2/Blueprint/Tank/UI/UI_TankZoomIn.UI_TankZoomIn_C" `_as플레이어_컨트롤러`))
      (set `self.UI_TankZoomIn` _returnvalue))
    (:`then_1`
      (`self.ZoomOut`))))

(event `Fire`
  (bind _scene (`self.Scene`))
  (if (`self.bFire`)
    (set `self.bFire` false)
    (`|SpawnActorFromClass` "/Game/KDT2/Blueprint/Tank/BP_Projectile.BP_Projectile_C" (`KismetMathLibrary.MakeTransform` (`SceneComponent.K2_GetComponentLocation` _scene) (`SceneComponent.K2_GetComponentRotation` _scene)) "AlwaysSpawn" "MultiplyWithRoot" self 5000.0 self)
    (`KismetSystemLibrary.Delay` 0.5)
    (set `self.bFire` true)))

(fn `UserConstructionScript`)

(fn `ZoomIn`
  (`ActorComponent.SetActive` (`self.ZoomCamera`) true false)
  (`ActorComponent.SetActive` (`self.Camera`) false false)
  (`UserWidget.AddToViewport` (`self.UI_TankZoomIn`) 0))

(fn `ZoomOut`
  (`ActorComponent.SetActive` (`self.ZoomCamera`) false false)
  (`ActorComponent.SetActive` (`self.Camera`) true false)
  (`Widget.RemoveFromParent` (`self.UI_TankZoomIn`)))